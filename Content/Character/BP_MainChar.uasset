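; BP_MainChar is the player-controlled main character, handling movement input and on-screen widget setup.
; On BeginPlay it adds the IMC_MainChar Enhanced Input context and puts a Text_Input widget on the viewport, provided a PlayerController possesses it.
; IA_Move drives movement along fixed world axes, with input X mapped to negative world X, independent of camera.
; It also records the input as Directionality and tracks whether move is held.
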(event `self.ReceiveBeginPlay`
  (bind _asplayer_controller (cast `PlayerController` (`self.GetController`)))
  (`EnhancedInputSubsystemInterface.AddMappingContext` (pcsubsystem `EnhancedInputLocalPlayerSubsystem` _asplayer_controller) "/Game/Character/Input/IMC_MainChar.IMC_MainChar" 0 (struct))
  (bind _returnvalue (`|CreateWidget` "/Game/Text_Input.Text_Input_C"))
  (`UserWidget.AddToViewport` _returnvalue 0))

(event `EnhancedInput|/Game/Character/Input/IA_Move`
  (params (ActionValue :type "Vector2D Structure") (ElapsedSeconds :type "Float (double-precision)") (TriggeredSeconds :type "Float (double-precision)") (InputAction :type "InputAction Object Reference" :default "/Game/Character/Input/IA_Move.IA_Move"))
  (:`Triggered`
    (`self.AddMovementInput` (-1.0 0.0 0.0) ActionValue_X)
    (`self.AddMovementInput` (0.0 1.0 0.0) ActionValue_Y)
    (set `self.Directionality` (`KismetMathLibrary.MakeVector2D` ActionValue_X ActionValue_Y)))
  (:`Started`
    (set `self.IsHoldingMove` true))
  (:`Completed`
    (set `self.IsHoldingMove` false)))

(fn `UserConstructionScript`)